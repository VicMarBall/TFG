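; BP_BasicAbility_Enhanced is the projectile actor for the enhanced basic ability VFX.
; On BeginPlay it activates its Niagara effect, zeroes the projectile movement's gravity and velocity, and sets a two-second lifespan.
; When its Sphere component hits, it prints the other actor's name, spawns the enhanced impact Niagara system at the hit location and destroys itself.
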(event OnComponentHit(Sphere)
  (params (HitComponent :type Primitive%20Component%20Object%20Reference) (OtherActor :type Actor%20Object%20Reference) (OtherComp :type Primitive%20Component%20Object%20Reference) (NormalImpulse :type Vector :default "0, 0, 0") (Hit :type Hit%20Result%20Structure%20%28by%20ref%29))
  (Development|PrintString (Utilities|GetDisplayName OtherActor))
  (Niagara|SpawnSystematLocation "/Game/AbilitiesVFXs/BasicAbility/Enhanced/FXS_BasicAbilityImpact_Enhanced.FXS_BasicAbilityImpact_Enhanced" (.location Hit) (.rotation (Transformation|GetActorTransform)))
  (Actor|DestroyActor))

(event EventBeginPlay
  (bind _projectilemovement (Variables|Default|GetProjectileMovement))
  (Components|Activation|SetActive (Variables|NiagaraActor|GetNiagaraComponent) true false)
  (Variables|/Script/Engine.ProjectileMovementComponent|SetProjectileGravityScale _projectilemovement 0.0)
  (Variables|/Script/Engine.MovementComponent|SetVelocity _projectilemovement "0, 0, 0")
  (Actor|SetLifeSpan 2.0))

(fn ConstructionScript)