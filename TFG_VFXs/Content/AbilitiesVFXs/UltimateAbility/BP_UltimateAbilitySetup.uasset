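; BP_UltimateAbilitySetup drives the ultimate ability effect, moving a projectile along a spline and triggering its explosion.
; Tick calls Play on a timeline whose Progress track positions and rotates the child actor projectile from the spline's world-space transform at that time.
; The timeline's Explosion event casts the child actor to BP_UltimateAbilityProjectile and calls OnSpawnExplosion with this setup actor's transform.
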(event EventTick
  (params (DeltaSeconds :type Float%20%28single-precision%29))
  (bind _progress (Timeline|Timeline Play)
    (:Update
      (Transformation|SetWorldTransform (Variables|Default|GetBP_UltimateAbilityProjectile) (Math|Transform|MakeTransform (Spline|GetLocationatTime (Variables|Default|GetSpline) _progress "World" false) (Class|SplineComponent|GetRotationatTime (Variables|Default|GetSpline) _progress "World" false) "1.000000,1.000000,1.000000") false false))
    (:Explosion
      (bind _asbp_ultimate_ability_projectile (Utilities|Casting|CastToBP_UltimateAbilityProjectile (Variables|/Script/Engine.ChildActorComponent|GetChildActor (Variables|Default|GetBP_UltimateAbilityProjectile))))
      (Default|OnSpawnExplosion _asbp_ultimate_ability_projectile (Transformation|GetActorTransform)))))

(fn ConstructionScript)