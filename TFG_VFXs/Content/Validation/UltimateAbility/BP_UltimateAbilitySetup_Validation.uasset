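; Validation actor for an ultimate ability that flies a child-actor projectile along a spline and triggers its explosion.
; BeginPlay snaps the projectile to the spline start, then Tick calls Play on a timeline whose Progress drives location and rotation along the path.
; The timeline's Explosion event spawns the explosion with this actor's transform, not the projectile's.
; On finish, it deactivates the projectile's Niagara effect and destroys itself after a delay.
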(event EventBeginPlay
  (Transformation|SetWorldTransform (Variables|Default|GetBP_UltimateAbilityProjectile) (Math|Transform|MakeTransform (Spline|GetLocationatTime (Variables|Default|GetSpline) 0.0 "World" false) (Class|SplineComponent|GetRotationatTime (Variables|Default|GetSpline) 0.0 "World" false) "1.000000,1.000000,1.000000") false false))

(event EventTick
  (params (DeltaSeconds :type Float%20%28single-precision%29))
  (bind _progress (Timeline|Timeline Play)
    (:Update
      (Transformation|SetWorldTransform (Variables|Default|GetBP_UltimateAbilityProjectile) (Math|Transform|MakeTransform (Spline|GetLocationatTime (Variables|Default|GetSpline) _progress "World" false) (Class|SplineComponent|GetRotationatTime (Variables|Default|GetSpline) _progress "World" false) "1.000000,1.000000,1.000000") false false))
    (:Finished
      (bind _asbp_ultimate_ability_projectile_validation (Utilities|Casting|CastToBP_UltimateAbilityProjectile_Validation (Variables|/Script/Engine.ChildActorComponent|GetChildActor (Variables|Default|GetBP_UltimateAbilityProjectile))))
      (Components|Activation|Deactivate (Variables|/Script/Niagara.NiagaraActor|GetNiagaraComponent _asbp_ultimate_ability_projectile_validation))
      (Utilities|FlowControl|Delay 3.0)
      (Actor|DestroyActor))
    (:Explosion
      (bind _asbp_ultimate_ability_projectile_validation_2 (Utilities|Casting|CastToBP_UltimateAbilityProjectile_Validation (Variables|/Script/Engine.ChildActorComponent|GetChildActor (Variables|Default|GetBP_UltimateAbilityProjectile))))
      (Default|OnSpawnExplosion _asbp_ultimate_ability_projectile_validation_2 (Transformation|GetActorTransform)))))

(fn ConstructionScript)