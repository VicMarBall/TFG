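; BP_BasicAbility_Regular_Validation is an actor for the regular basic ability in the Validation folder, built from a Niagara effect, projectile movement and a sphere component.
; On BeginPlay it activates the effect, zeroes the projectile's gravity and velocity so it starts stationary, and sets a short life span.
; Hit deactivates movement, effect and sphere, then destroys the actor after a delay.
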(event EventBeginPlay
  (bind _projectilemovement (Variables|Default|GetProjectileMovement))
  (Components|Activation|SetActive (Variables|NiagaraActor|GetNiagaraComponent) true false)
  (Variables|/Script/Engine.ProjectileMovementComponent|SetProjectileGravityScale _projectilemovement 0.0)
  (Variables|/Script/Engine.MovementComponent|SetVelocity _projectilemovement "0, 0, 0")
  (Actor|SetLifeSpan 2.0))

(event Collision|EventHit
  (params (MyComp :type Primitive%20Component%20Object%20Reference) (Other :type Actor%20Object%20Reference) (OtherComp :type Primitive%20Component%20Object%20Reference) (bSelfMoved :type Boolean) (HitLocation :type Vector :default "0, 0, 0") (HitNormal :type Vector :default "0, 0, 0") (NormalImpulse :type Vector :default "0, 0, 0") (Hit :type Hit%20Result%20Structure%20%28by%20ref%29))
  (Components|Activation|Deactivate (Variables|Default|GetProjectileMovement))
  (Components|Activation|Deactivate (Variables|NiagaraActor|GetNiagaraComponent))
  (Components|Activation|Deactivate (Variables|Default|GetSphere))
  (Utilities|FlowControl|Delay 2.0)
  (Actor|DestroyActor))

(fn ConstructionScript)